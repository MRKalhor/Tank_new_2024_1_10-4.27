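; BP_MyPawn_Tank is a tank pawn built on a four-wheel vehicle movement component.
; Each tick it casts its Audio component to FXSystemComponent and, if that succeeds, writes forward speed to the "rms" float parameter.
; Red material swaps on body and turret and two camera view-target switches are unwired, and the other events are empty.
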(event Custom|RBC_changematerial)

(event EventBeginPlay
  ;[1 1 1] Camera 1
)

(event Collision|EventActorBeginOverlap
  (params (OtherActor :type Actor%20Object%20Reference)))

(event EventTick
  (params (DeltaSeconds :type Float%20%28single-precision%29))
  (bind _asfxsystem_component (Utilities|Casting|CastToFXSystemComponent (Variables|Default|GetAudio)))
  (Effects|Components|ParticleSystem|SetFloatParameter _asfxsystem_component "rms" (Class|WheeledVehicleMovementComponent|GetForwardSpeed (Variables|Default|GetWheeledVehicleMovementComponent4W))))

(event Input|MouseEvents|RightMouseButton
  (params (Key :type Key%20Structure :default "None"))
  ;[1 1 1] Camera 2
)

(fn ConstructionScript)